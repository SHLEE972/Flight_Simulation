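; Player-controlled aircraft Blueprint flown through a JSBSim movement component.
; Enhanced Input drives yoke, rudder, four throttles, parking brake and timeline-animated landing gear, writing flight commands and mirroring most onto the CommercialPlane animation Blueprint.
; One camera switches between cockpit and third-person mounts, with orbit, zoom and reset in third person.
; Tick levels the third-person rig against a planet-centre up vector and sends latitude and longitude to a widget.
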(event Custom|Set%20Throttle%20Value
  (params (Throttle%20Index :type Integer) (Throttle%20Value :type Float%20%28double-precision%29))
  (bind _throttlevalues (Variables|Default|GetThrottleValues))
  (Utilities|Struct|SetmembersinEngineCommand (Utilities|Array|Get(acopy) (Variables|/Script/JSBSimFlightDynamicsModel.JSBSimMovementComponent|GetEngineCommands (Variables|Default|GetJSBSimMovement)) Throttle%20Index) Throttle%20Value)
  (bind _animblueprintreference (Utilities|GetAnimBlueprintRef))
  (Variables|/Game/CommercialPlane/Meshes/CommercialPlane_AnimBlueprint.CommercialPlane_AnimBlueprint_C|SetLeftEngine _animblueprintreference (+ (Utilities|Array|Get(acopy) _throttlevalues) (Utilities|Array|Get(acopy) _throttlevalues)))
  (Variables|/Game/CommercialPlane/Meshes/CommercialPlane_AnimBlueprint.CommercialPlane_AnimBlueprint_C|SetRightEngine _animblueprintreference (+ (Utilities|Array|Get(acopy) _throttlevalues) (Utilities|Array|Get(acopy) _throttlevalues))))

(event Custom|AlignThirdPersonCamera
  (bind _returnvalue (Transformation|GetActorLocation))
  (bind _returnvalue_2 (Math|Vector|MakeVector 0.0 0.0 -6.38e+08))
  (bind _returnvalue_3 (- _returnvalue _returnvalue_2))
  (bind _returnvalue_4 (Math|Vector|Normalize _returnvalue_3))
  (Transformation|SetWorldRotation (Variables|Default|GetThirdPersonViewOrigin) (Math|Rotator|MakeRotfromXZ (Math|Vector|ProjectVectorontoPlane (Transformation|GetActorForwardVector) _returnvalue_4) _returnvalue_4) false false))

(event Custom|RefreshWidget
  (bind _widgetreference (Variables|Default|GetWidgetReference))
  (bind _jsbsimmovement (Variables|Default|GetJSBSimMovement))
  (bind _aircraftstate (Variables|/Script/JSBSimFlightDynamicsModel.JSBSimMovementComponent|GetAircraftState _jsbsimmovement))
  (bind (_latitude _longitude) (Utilities|Struct|BreakAircraftState _aircraftstate))
  (Utilities|IsValid _widgetreference
    (:Is%20Valid
      (Default|SetCoordinate _widgetreference _latitude _longitude))))

(event Custom|ToggleParkingBrake
  (bind _jsbsimmovement (Variables|Default|GetJSBSimMovement))
  ;[1 1 1] fright
  (bind _structout (Utilities|Struct|SetmembersinFlightControlCommands (Variables|/Script/JSBSimFlightDynamicsModel.JSBSimMovementComponent|GetCommands (Variables|Default|GetJSBSimMovement)) (- 1.0 (Utilities|Struct|BreakFlightControlCommands (Variables|/Script/JSBSimFlightDynamicsModel.JSBSimMovementComponent|GetCommands _jsbsimmovement)))))
  (Variables|/Script/JSBSimFlightDynamicsModel.JSBSimMovementComponent|SetCommands _jsbsimmovement _structout))

(event Input|EnhancedActionEvents|EnhancedInputActionIA_Toggle_Camera
  (params (ActionValue :type Boolean) (ElapsedSeconds :type Float%20%28double-precision%29) (TriggeredSeconds :type Float%20%28double-precision%29) (InputAction :type Input%20Action%20Object%20Reference :default "/Game/input/IA_Toggle_Camera.IA_Toggle_Camera"))
  (bind _camera (Variables|Default|GetCamera))
  (:Started
    (bind _isa (Utilities|FlowControl|FlipFlop)
      (:A
        _)
      (:B
        _))
    (bind _output_get (Variables|Default|SetThirdPersonView _isa))
    (Transformation|AttachComponentToComponent _camera (select _output_get (Variables|Default|GetThirdPersonViewTransform) (Variables|Default|GetCockpitViewTransform)) "None" "SnapToTarget" "SnapToTarget" "KeepWorld" true)
    (Transformation|SetRelativeTransform _camera (Math|Transform|MakeTransform "0, 0, 0") false false)
    (Camera|SetFieldOfView (Variables|Default|GetCamera) (select (Variables|Default|GetThirdPersonView) (Variables|Default|GetFieldOfView) 9e+01))))

(event Input|EnhancedActionEvents|EnhancedInputActionIA_LotateCamera
  (params (ActionValue :type Vector%202D%20Structure) (ElapsedSeconds :type Float%20%28double-precision%29) (TriggeredSeconds :type Float%20%28double-precision%29) (InputAction :type Input%20Action%20Object%20Reference :default "/Game/input/IA_LotateCamera.IA_LotateCamera"))
  (bind (_x _y) (Math|Vector2D|BreakVector2D ActionValue))
  (bind _thirdpersonpitchorigin (Variables|Default|GetThirdPersonPitchOrigin))
  (if (and (Variables|Default|GetWheelClickDown) (Variables|Default|GetThirdPersonView))
    (Transformation|AddRelativeRotation (Variables|Default|GetThirdPersonYawOrigin) (Math|Rotator|MakeRotator 0.0 0.0 _x) false false)
    (Transformation|SetRelativeRotation _thirdpersonpitchorigin (Math|Rotator|MakeRotator 0.0 (Math|Float|Clamp(Float) (+ (.Pitch (Math|Rotator|BreakRotator (Variables|/Script/Engine.SceneComponent|GetRelativeRotation _thirdpersonpitchorigin))) _y) -8e+01 8e+01) 0.0) false false)))

(event Input|EnhancedActionEvents|EnhancedInputActionIA_Zoom
  (params (ActionValue :type Float%20%28double-precision%29) (ElapsedSeconds :type Float%20%28double-precision%29) (TriggeredSeconds :type Float%20%28double-precision%29) (InputAction :type Input%20Action%20Object%20Reference :default "/Game/input/IA_Zoom.IA_Zoom"))
  (if (Variables|Default|GetThirdPersonView)
    (bind _output_get (Variables|Default|SetFieldOfView (Math|Float|Clamp(Float) (+ (* ActionValue -3.0) (Variables|Default|GetFieldOfView)) 45.0 9e+01)))
    (Camera|SetFieldOfView (Variables|Default|GetCamera) _output_get)))

(event Input|EnhancedActionEvents|EnhancedInputActionIA_ResetCamera
  (params (ActionValue :type Boolean) (ElapsedSeconds :type Float%20%28double-precision%29) (TriggeredSeconds :type Float%20%28double-precision%29) (InputAction :type Input%20Action%20Object%20Reference :default "/Game/input/IA_ResetCamera.IA_ResetCamera"))
  (:Started
    (if (Variables|Default|GetThirdPersonView)
      (Transformation|SetRelativeRotation (Variables|Default|GetThirdPersonPitchOrigin) "0, 0, 0" false false)
      (bind _output_get (Variables|Default|SetFieldOfView 9e+01))
      (Camera|SetFieldOfView (Variables|Default|GetCamera) _output_get))))

(event Input|EnhancedActionEvents|EnhancedInputActionIA_EnableCamera
  (params (ActionValue :type Boolean) (ElapsedSeconds :type Float%20%28double-precision%29) (TriggeredSeconds :type Float%20%28double-precision%29) (InputAction :type Input%20Action%20Object%20Reference :default "/Game/input/IA_EnableCamera.IA_EnableCamera"))
  (:Started
    (Variables|Default|SetWheelClickDown ActionValue :!label _label))
  (:Completed
    (goto _label)))

(event EventBeginPlay
  (bind _returnvalue (Game|GetPlayerController 0))
  (bind _jsbsimmovement (Variables|Default|GetJSBSimMovement))
  (bind _returnvalue_2 (PlayerController|LocalPlayerSubsystems|GetEnhancedInputLocalPlayerSubsystem _returnvalue))
  ;[1 1 1] initialize input
  (Input|AddMappingContext _returnvalue_2 "/Game/input/IAC_Aircraft_Control.IAC_Aircraft_Control" 0 "(bIgnoreAllPressedKeysUntilRelease=True,bForceImmediately=False,bNotifyUserSettings=False)")
  (Input|AddMappingContext _returnvalue_2 "/Game/input/IAC_OtherControl.IAC_OtherControl" 0 "(bIgnoreAllPressedKeysUntilRelease=True,bForceImmediately=False,bNotifyUserSettings=False)")
  ;[1 1 1] fright
  (bind _structout (Utilities|Struct|SetmembersinFlightControlCommands (Variables|/Script/JSBSimFlightDynamicsModel.JSBSimMovementComponent|GetCommands (Variables|Default|GetJSBSimMovement)) (- 1.0 (Utilities|Struct|BreakFlightControlCommands (Variables|/Script/JSBSimFlightDynamicsModel.JSBSimMovementComponent|GetCommands _jsbsimmovement)))))
  (Variables|/Script/JSBSimFlightDynamicsModel.JSBSimMovementComponent|SetCommands _jsbsimmovement _structout))

(event EventTick
  (params (DeltaSeconds :type Float%20%28single-precision%29))
  (CallFunction|AlignThirdPersonCamera)
  (CallFunction|RefreshWidget))

(event Input|EnhancedActionEvents|EnhancedInputActionIA_Parking_Break
  (params (ActionValue :type Boolean) (ElapsedSeconds :type Float%20%28double-precision%29) (TriggeredSeconds :type Float%20%28double-precision%29) (InputAction :type Input%20Action%20Object%20Reference :default "/Game/input/IA_Parking_Break.IA_Parking_Break"))
  (:Started
    (if ActionValue
      (CallFunction|ToggleParkingBrake))))

(event Input|EnhancedActionEvents|EnhancedInputActionIA_Throttle_First
  (params (ActionValue :type Float%20%28double-precision%29) (ElapsedSeconds :type Float%20%28double-precision%29) (TriggeredSeconds :type Float%20%28double-precision%29) (InputAction :type Input%20Action%20Object%20Reference :default "/Game/input/IA_Throttle_First.IA_Throttle_First"))
  (bind (_throttleindex _outputindex) (Utilities|SetLocalThrottleValue ActionValue))
  (CallFunction|SetThrottleValue _outputindex _throttleindex))

(event Input|EnhancedActionEvents|EnhancedInputActionIA_Throttle_Second
  (params (ActionValue :type Float%20%28double-precision%29) (ElapsedSeconds :type Float%20%28double-precision%29) (TriggeredSeconds :type Float%20%28double-precision%29) (InputAction :type Input%20Action%20Object%20Reference :default "/Game/input/IA_Throttle_Second.IA_Throttle_Second"))
  (bind (_throttleindex _outputindex) (Utilities|SetLocalThrottleValue ActionValue 1))
  (CallFunction|SetThrottleValue _outputindex _throttleindex))

(event Input|EnhancedActionEvents|EnhancedInputActionIA_Throttle_Third
  (params (ActionValue :type Float%20%28double-precision%29) (ElapsedSeconds :type Float%20%28double-precision%29) (TriggeredSeconds :type Float%20%28double-precision%29) (InputAction :type Input%20Action%20Object%20Reference :default "/Game/input/IA_Throttle_Third.IA_Throttle_Third"))
  (bind (_throttleindex _outputindex) (Utilities|SetLocalThrottleValue ActionValue 2))
  (CallFunction|SetThrottleValue _outputindex _throttleindex))

(event Input|EnhancedActionEvents|EnhancedInputActionIA_Throttle_Fourth
  (params (ActionValue :type Float%20%28double-precision%29) (ElapsedSeconds :type Float%20%28double-precision%29) (TriggeredSeconds :type Float%20%28double-precision%29) (InputAction :type Input%20Action%20Object%20Reference :default "/Game/input/IA_Throttle_Fourth.IA_Throttle_Fourth"))
  (bind (_throttleindex _outputindex) (Utilities|SetLocalThrottleValue ActionValue 3))
  (CallFunction|SetThrottleValue _outputindex _throttleindex))

(event Input|EnhancedActionEvents|EnhancedInputActionIA_Yoke
  (params (ActionValue :type Vector%202D%20Structure) (ElapsedSeconds :type Float%20%28double-precision%29) (TriggeredSeconds :type Float%20%28double-precision%29) (InputAction :type Input%20Action%20Object%20Reference :default "/Game/input/IA_Yoke.IA_Yoke"))
  (bind (_x _y) (Math|Vector2D|BreakVector2D ActionValue))
  (bind _jsbsimmovement (Variables|Default|GetJSBSimMovement))
  (:Triggered
    (bind _structout (Utilities|Struct|SetmembersinFlightControlCommands (Variables|/Script/JSBSimFlightDynamicsModel.JSBSimMovementComponent|GetCommands _jsbsimmovement) _x _y :!label _label))
    (Variables|/Script/JSBSimFlightDynamicsModel.JSBSimMovementComponent|SetCommands _jsbsimmovement _structout)
    (bind _animblueprintreference (Utilities|GetAnimBlueprintRef))
    (Variables|/Game/CommercialPlane/Meshes/CommercialPlane_AnimBlueprint.CommercialPlane_AnimBlueprint_C|SetAileronLeft _animblueprintreference (+ (* (* _x -1.0) 5e+01) 5e+01))
    (Variables|/Game/CommercialPlane/Meshes/CommercialPlane_AnimBlueprint.CommercialPlane_AnimBlueprint_C|SetAileronRight _animblueprintreference (+ (* _x 5e+01) 5e+01))
    (Variables|/Game/CommercialPlane/Meshes/CommercialPlane_AnimBlueprint.CommercialPlane_AnimBlueprint_C|SetFlapsTail _animblueprintreference (* _y -45.0)))
  (:Completed
    (goto _label)))

(event Input|EnhancedActionEvents|EnhancedInputActionIA_Landing_Gear
  (params (ActionValue :type Boolean) (ElapsedSeconds :type Float%20%28double-precision%29) (TriggeredSeconds :type Float%20%28double-precision%29) (InputAction :type Input%20Action%20Object%20Reference :default "/Game/input/IA_Landing_Gear.IA_Landing_Gear"))
  (bind _jsbsimmovement (Variables|Default|GetJSBSimMovement))
  (:Started
    (if (not (Variables|Default|GetLandingGearOperating))
      (Variables|Default|SetLandingGearOperating true)
      (if (Math|Float|NearlyEqual(Float) (Utilities|Struct|BreakFlightControlCommands (Variables|/Script/JSBSimFlightDynamicsModel.JSBSimMovementComponent|GetCommands (Variables|Default|GetJSBSimMovement))) 1.0 1e-06)
        (bind (_direction _landinggeardownamount _noselandinggearretractamount _noselandinggeardooropenamount) (Timeline|LandingGearUp PlayFromStart)
          (:Update
            (bind _structout (Utilities|Struct|SetmembersinFlightControlCommands (Variables|/Script/JSBSimFlightDynamicsModel.JSBSimMovementComponent|GetCommands _jsbsimmovement) _landinggeardownamount))
            (Variables|/Script/JSBSimFlightDynamicsModel.JSBSimMovementComponent|SetCommands _jsbsimmovement _structout)
            (bind _animblueprintreference (Utilities|GetAnimBlueprintRef))
            (Variables|/Game/CommercialPlane/Meshes/CommercialPlane_AnimBlueprint.CommercialPlane_AnimBlueprint_C|SetFrontGearRetract _animblueprintreference _noselandinggearretractamount)
            (Variables|/Game/CommercialPlane/Meshes/CommercialPlane_AnimBlueprint.CommercialPlane_AnimBlueprint_C|SetFrontGearDoor _animblueprintreference _noselandinggeardooropenamount)
            (Variables|/Game/CommercialPlane/Meshes/CommercialPlane_AnimBlueprint.CommercialPlane_AnimBlueprint_C|SetMainGearRetract _animblueprintreference _noselandinggearretractamount)
            (Variables|/Game/CommercialPlane/Meshes/CommercialPlane_AnimBlueprint.CommercialPlane_AnimBlueprint_C|SetMainGearDoorBay _animblueprintreference _noselandinggeardooropenamount))
          (:Finished
            (Variables|Default|SetLandingGearOperating false)))
        (else
          (Timeline|LandingGearUp ReverseFromEnd))))))

(event Input|EnhancedActionEvents|EnhancedInputActionIA_Rudder
  (params (ActionValue :type Float%20%28double-precision%29) (ElapsedSeconds :type Float%20%28double-precision%29) (TriggeredSeconds :type Float%20%28double-precision%29) (InputAction :type Input%20Action%20Object%20Reference :default "/Game/input/IA_Rudder.IA_Rudder"))
  (bind _jsbsimmovement (Variables|Default|GetJSBSimMovement))
  (:Triggered
    (bind _structout (Utilities|Struct|SetmembersinFlightControlCommands (Variables|/Script/JSBSimFlightDynamicsModel.JSBSimMovementComponent|GetCommands _jsbsimmovement) ActionValue :!label _label))
    (Variables|/Script/JSBSimFlightDynamicsModel.JSBSimMovementComponent|SetCommands _jsbsimmovement _structout)
    (bind _animblueprintreference (Utilities|GetAnimBlueprintRef))
    (Variables|/Game/CommercialPlane/Meshes/CommercialPlane_AnimBlueprint.CommercialPlane_AnimBlueprint_C|SetFlapsTopTail _animblueprintreference (* ActionValue -45.0)))
  (:Completed
    (goto _label)))

(fn ConstructionScript)