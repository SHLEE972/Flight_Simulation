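; GameModeFlightScene is the game mode Blueprint for a flight scene, setting up the player's aircraft and main UI when play begins.
; On BeginPlay it casts the player pawn to BP_Aircraft and turns off debug drawing on its JSBSim movement component.
; It then creates the WBP_Main widget, adds it to the viewport and hands the aircraft a reference to it.
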(event EventBeginPlay
  (bind _asbp_aircraft (Utilities|Casting|CastToBP_Aircraft (Game|Player|GetPlayerPawn 0)))
  (bind _output_get (Variables|Default|SetBPAircraft _asbp_aircraft))
  (Variables|/Script/JSBSimFlightDynamicsModel.JSBSimMovementComponent|SetDrawDebug (Variables|/Game/Blueprints/BP_Aircraft.BP_Aircraft_C|GetJSBSimMovement _output_get) false)
  (bind _returnvalue (UserInterface|CreateWidget "/Game/WidgetBluePrints/WBP_Main.WBP_Main_C")) ; CreateWidget
  (bind _output_get_2 (Variables|Default|SetMainWidget _returnvalue)) ; Promote to Widget
  (UserInterface|Viewport|AddtoViewport _output_get_2 0)
  (Variables|/Game/Blueprints/BP_Aircraft.BP_Aircraft_C|SetWidgetReference (Variables|Default|GetBPAircraft) (Variables|Default|GetMainWidget)))

(fn ConstructionScript)